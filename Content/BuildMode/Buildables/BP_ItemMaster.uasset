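; BP_ItemMaster is a build mode buildable item, apparently the base class, that carries a static mesh and part properties.
; Events set the mesh and flag the item as connected.
; Getters expose the connected state, durability, weight, speed multiplier, and cockpit, engine and wheel properties, plus all box components.
; IsBuildFinished always returns false, and the construction script, overlap and tick are empty.
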(event `/Game/BuildMode/ItemsInterface.SetConnected`
  (set `self.Connected?` true))

(event `/Game/BuildMode/ItemsInterface.SetMesh`
  (params (Mesh :type "StaticMesh Object Reference"))
  (`StaticMeshComponent.SetStaticMesh` (`self.StaticMesh`) Mesh))

(fn `GetConnected`
  (returns (Connected :type Boolean))
  (return (`self.Connected?`)))

(fn `IsBuildFinished`
  (returns (IsFinished :type Boolean))
  (return false))

(fn `ItemProperties`
  (returns (Durability :type "Float (double-precision)") (Weight :type "Float (double-precision)") (SpeedMultiplier :type "Float (double-precision)") (Connected :type Boolean) (Cockpit :type Boolean) (Engine :type Boolean) (Wheel :type Boolean))
  (return (`self.Durability`) (`self.Weight`) (`self.SpeedMultiplier`) (`self.Connected?`) (`self.Cockpit?`) (`self.Engine?`) (`self.Wheel?`)))

(fn `ReturnBoxes`
  (returns (Boxes :type "Array of BoxComponent Object Reference"))
  (return (`self.K2_GetComponentsByClass` "/Script/Engine.BoxComponent")))

(fn `UserConstructionScript`)