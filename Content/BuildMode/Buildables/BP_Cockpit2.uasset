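; BP_Cockpit2 is a buildable cockpit piece for build mode.
; On BeginPlay it sets CockpitBuild to true on the BuildComponent of the player's BP_ThirdPersonCharacter.
; ReturnBoxes exposes the piece's set of box references.
; GetConnected, IsBuildFinished and ItemProperties return only false or zero values, so even the Cockpit property reads false.
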(event `self.ReceiveBeginPlay`
  (bind _asbp_third_person_character (cast `/Game/ThirdPerson/Blueprints/BP_ThirdPersonCharacter` (`GameplayStatics.GetPlayerCharacter` 0)))
  (set `/Game/BuildMode/BuildComponent.CockpitBuild` true (`/Game/ThirdPerson/Blueprints/BP_ThirdPersonCharacter.BuildComponent` _asbp_third_person_character)))

(fn `GetConnected`
  (returns (Connected :type Boolean))
  (return false))

(fn `IsBuildFinished`
  (returns (IsFinished :type Boolean))
  (return false))

(fn `ItemProperties`
  (returns (Durability :type "Float (double-precision)") (Weight :type "Float (double-precision)") (SpeedMultiplier :type "Float (double-precision)") (Connected :type Boolean) (Cockpit :type Boolean) (Engine :type Boolean) (Wheel :type Boolean))
  (return 0.0 0.0 0.0 false false false false))

(fn `ReturnBoxes`
  (returns (Boxes :type "Array of BoxComponent Object Reference"))
  (return (`|MakeArray` (`self.Box`) (`self.Box1`) (`self.Box2`) (`self.Box3`) (`self.Box4`) (`self.Box5`) (`self.Box6`) (`self.Box7`) (`self.Box8`) (`self.Box9`) (`self.Box10`) (`self.Box11`))))

(fn `UserConstructionScript`)