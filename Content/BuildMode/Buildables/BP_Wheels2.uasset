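; BP_Wheels2 is a buildable wheels Blueprint for build mode, with no active event or construction logic of its own.
; It exposes six box components as an array through ReturnBoxes.
; IsBuildFinished and ReturnDurability are placeholders that always return false and zero.
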(fn `IsBuildFinished`
  (returns (IsFinished :type Boolean))
  (return false))

(fn `ReturnBoxes`
  (returns (Boxes :type "Array of BoxComponent Object Reference"))
  (return (`|MakeArray` (`self.Box`) (`self.Box1`) (`self.Box2`) (`self.Box3`) (`self.Box4`) (`self.Box5`))))

(fn `ReturnDurability`
  (returns (ReturnValue :type "Float (double-precision)"))
  (return 0.0))

(fn `UserConstructionScript`)