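; BP_Cube is a test buildable cube for build mode, with a static mesh that the SetMesh event can swap.
; It sets Connected on BeginPlay and reports it through ItemProperties, alongside durability, weight, speed multiplier and part-type values.
; ReturnBoxes exposes its box components, while GetConnected and IsBuildFinished are stubs that always return false, so GetConnected ignores the Connected variable.
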(event `self.ReceiveBeginPlay`
  (set `self.Connected?` true))

(event `/Game/BuildMode/ItemsInterface.SetMesh`
  (params (Mesh :type "StaticMesh Object Reference"))
  (`StaticMeshComponent.SetStaticMesh` (`self.StaticMeshComponent`) Mesh))

(fn `GetConnected`
  (returns (Connected :type Boolean))
  (return false))

(fn `IsBuildFinished`
  (returns (IsFinished :type Boolean))
  (return false))

(fn `ItemProperties`
  (returns (Durability :type "Float (double-precision)") (Weight :type "Float (double-precision)") (SpeedMultiplier :type "Float (double-precision)") (Connected :type Boolean) (Cockpit :type Boolean) (Engine :type Boolean) (Wheel :type Boolean))
  (return (`self.Durability`) (`self.Weight`) (`self.SpeedMultiplier`) (`self.Connected?`) (`self.Cockpit?`) (`self.Engine?`) (`self.Wheel?`)))

(fn `ReturnBoxes`
  (returns (Boxes :type "Array of BoxComponent Object Reference"))
  (return (`self.K2_GetComponentsByClass` "/Script/Engine.BoxComponent")))

(fn `UserConstructionScript`)