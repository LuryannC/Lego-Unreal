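; BP_Items is a build mode buildable Blueprint that provides placeholder query functions, apparently as a base for vehicle parts such as cockpits, engines and wheels.
; Its connection and build-finished checks return false, and ItemProperties returns zeroed stats and false part-type flags.
; ReturnBoxes exposes six box references as an array, while the event graph and construction script do nothing.
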(event `self.ReceiveBeginPlay`)

(fn `GetConnected`
  (returns (Connected :type Boolean))
  (return false))

(fn `IsBuildFinished`
  (returns (IsFinished :type Boolean))
  (return false))

(fn `ItemProperties`
  (returns (Durability :type "Float (double-precision)") (Weight :type "Float (double-precision)") (SpeedMultiplier :type "Float (double-precision)") (Connected :type Boolean) (Cockpit :type Boolean) (Engine :type Boolean) (Wheel :type Boolean))
  (return 0.0 0.0 0.0 false false false false))

(fn `ReturnBoxes`
  (returns (Boxes :type "Array of BoxComponent Object Reference"))
  (return (`|MakeArray` (`self.Box`) (`self.Box1`) (`self.Box2`) (`self.Box3`) (`self.Box4`) (`self.Box5`))))

(fn `UserConstructionScript`)